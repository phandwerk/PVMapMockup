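; WallMountedLight is a wall-mounted lamp actor for the OldTown environment, pairing a PotLight mesh with a point light.
; The construction script creates a dynamic StreetLamp_Emissive material on the mesh and applies the shadow-casting setting to the light.
; A LightToggle flag drives both emissive strength and light brightness from one Intensity value, scaled up for the light, or zeroes both when off.
; The event graph holds no active logic.
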(fn `UserConstructionScript`
  (bind _intensity (`self.Intensity`))
  (bind _dmi (`self.DMI`))
  (bind _pointlight (`self.PointLight`))
  (bind _returnvalue (`PrimitiveComponent.CreateDynamicMaterialInstance` (`self.PotLight`) 0 "/Game/OldTown/Materials/StreetLamp_Emissive.StreetLamp_Emissive"))
  (set `self.DMI` _returnvalue)
  (`LightComponentBase.SetCastShadows` (`self.PointLight`) (`self.Cast Shadows`))
  (if (`self.Light Toggle`)
    (`MaterialInstanceDynamic.SetScalarParameterValue` _dmi "Emissive Strength" _intensity)
    (`LightComponent.SetIntensity` _pointlight (* _intensity 250.0))
    (else
      (`MaterialInstanceDynamic.SetScalarParameterValue` _dmi "Emissive Strength" 0.0)
      (`LightComponent.SetIntensity` _pointlight 0.0))))