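; Traffic light prop Blueprint that cycles red, green and yellow signals and carries optional street lamps.
; The construction script creates a dynamic material instance on the mesh and uses LightsOnoff to set the streetlight glow and two spotlights.
; BeginPlay runs an endless timed Delay loop that switches each colored light and its material parameter together.
; LightSequence picks whether the loop starts on red or green, with red lasting as long as green plus yellow.
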(event `self.ReceiveBeginPlay`
  (bind _redlight (`self.RedLight`))
  (bind _yellowlight (`self.YellowLight`))
  (bind _dmi (`self.DMI`))
  (bind _greenlight (`self.GreenLight`))
  (bind _redlight_2 (`self.RedLight`))
  (bind _yellowlight_2 (`self.YellowLight`))
  (bind _greenlight_2 (`self.GreenLight`))
  (if (`self.LightSequence`)
    (`LightComponent.SetIntensity` _redlight_2 1000.0 :!label _label)
    (`MaterialInstanceDynamic.SetScalarParameterValue` _dmi "Redlight" 1.0)
    (`KismetSystemLibrary.Delay` 30.0)
    (`MaterialInstanceDynamic.SetScalarParameterValue` _dmi "Redlight" 0.0)
    (`LightComponent.SetIntensity` _redlight_2 0.0)
    (`LightComponent.SetIntensity` _greenlight_2 1000.0)
    (`MaterialInstanceDynamic.SetScalarParameterValue` _dmi "Greenlight" 1.0)
    (`KismetSystemLibrary.Delay` 25.0)
    (`MaterialInstanceDynamic.SetScalarParameterValue` _dmi "Greenlight" 0.0)
    (`LightComponent.SetIntensity` _greenlight_2 0.0)
    (`LightComponent.SetIntensity` _yellowlight_2 1000.0)
    (`MaterialInstanceDynamic.SetScalarParameterValue` _dmi "Yellowlight" 1.0)
    (`KismetSystemLibrary.Delay` 5.0)
    (`MaterialInstanceDynamic.SetScalarParameterValue` _dmi "Yellowlight" 0.0)
    (`LightComponent.SetIntensity` _yellowlight_2 0.0)
    (goto _label)
    (else
      (`LightComponent.SetIntensity` _greenlight 1000.0 :!label _label_2)
      (`MaterialInstanceDynamic.SetScalarParameterValue` _dmi "Greenlight" 1.0)
      (`KismetSystemLibrary.Delay` 25.0)
      (`MaterialInstanceDynamic.SetScalarParameterValue` _dmi "Greenlight" 0.0)
      (`LightComponent.SetIntensity` _greenlight 0.0)
      (`LightComponent.SetIntensity` _yellowlight 1000.0)
      (`MaterialInstanceDynamic.SetScalarParameterValue` _dmi "Yellowlight" 1.0)
      (`KismetSystemLibrary.Delay` 5.0)
      (`MaterialInstanceDynamic.SetScalarParameterValue` _dmi "Yellowlight" 0.0)
      (`LightComponent.SetIntensity` _yellowlight 0.0)
      (`LightComponent.SetIntensity` _redlight 1000.0)
      (`MaterialInstanceDynamic.SetScalarParameterValue` _dmi "Redlight" 1.0)
      (`KismetSystemLibrary.Delay` 30.0)
      (`MaterialInstanceDynamic.SetScalarParameterValue` _dmi "Redlight" 0.0)
      (`LightComponent.SetIntensity` _redlight 0.0)
      (goto _label_2))))

(fn `UserConstructionScript`
  (bind _spotlight1 (`self.SpotLight1`))
  (bind _returnvalue (`PrimitiveComponent.CreateDynamicMaterialInstance` (`self.StaticMesh1`) 3 "/Game/UrbanCity/Materials/Props/prp_streetLight_Mat.prp_streetLight_Mat"))
  (set `self.DMI` _returnvalue)
  (if (`self.Lights on/off`)
    (`MaterialInstanceDynamic.SetScalarParameterValue` (`self.DMI`) "streetlight" 1.0))
  (if (`self.Lights on/off`)
    (`LightComponent.SetIntensity` _spotlight1 10000.0)
    (`LightComponent.SetIntensity` (`self.SpotLight2`) 10000.0)
    (else
      (`LightComponent.SetIntensity` _spotlight1 0.0)
      (`LightComponent.SetIntensity` (`self.SpotLight2`) 0.0))))