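; Street light prop Blueprint for UrbanCity that configures its lamp material and light in the construction script.
; It creates a dynamic instance of the street light material on a mesh slot and stores it as DMI.
; The LightsOn flag raises the material's streetlight parameter.
; A separate hard-coded true branch always sets the Light to full intensity, so its off path never runs.
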(fn `UserConstructionScript`
  (bind _light (`self.light`))
  (bind _returnvalue (`PrimitiveComponent.CreateDynamicMaterialInstance` (`self.StaticMesh1`) 2 "/Game/UrbanCity/Materials/Props/prp_streetLight_Mat.prp_streetLight_Mat"))
  (set `self.DMI` _returnvalue)
  (if (`self.LightsOn`)
    (`MaterialInstanceDynamic.SetScalarParameterValue` (`self.DMI`) "streetlight" 1.0))
  (if true
    (`LightComponent.SetIntensity` _light 5000.0)
    (else
      (`LightComponent.SetIntensity` _light 0.0))))